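; Course chrono actor, marked OLD, meant to show a countdown to the end of contest 1, stage 1 on a Text3D component.
; BeginPlay reads the stage EndTime from DTFlux data storage and splits the remaining time into hours, minutes and seconds, ignoring days.
; A timer function decrements these with manual rollover, without stopping at zero, and rewrites the text.
; Tick re-sets that one-second looping timer every frame, restarting it each time.
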(event `self.ReceiveBeginPlay`
  (bind _returnvalue (`DTFluxSubsystem.GetDataStorage` (subsystem `DTFluxSubsystem`)))
  (bind (_outstage _returnvalue_2) (`DTFluxDataStorage.GetStage` _returnvalue 1 1))
  (if _returnvalue_2
    (bind (_days _hours _minutes _seconds) (`KismetMathLibrary.BreakTimespan2` (- (`.EndTime` (break `DTFluxStage` _outstage)) (`KismetMathLibrary.Now`))))
    (set `self.CDHeure` _hours)
    (set `self.CDMinute` _minutes)
    (set `self.CDSecond` _seconds)))

(event `self.ReceiveTick`
  (params (DeltaSeconds :type "Float (single-precision)"))
  (`KismetSystemLibrary.K2_SetTimer` null "Timer Count Down" 1.0 true))

(fn `Timer Count Down`
  (if (== (`self.CDSecond`) 0)
    (if (== (`self.CDMinute`) 0)
      (set `self.CDMinute` 59)
      (set `self.CDSecond` 59)
      (set `self.CDHeure` (- (`self.CDHeure`) 1))
      (else
        (set `self.CDSecond` 59)
        (set `self.CDMinute` (- (`self.CDMinute`) 1))))
    (else
      (set `self.CDSecond` (- (`self.CDSecond`) 1))))
  (set `Text3DComponent.Text` (`KismetTextLibrary.Conv_StringToText` (`KismetStringLibrary.Concat_StrStr` (`KismetStringLibrary.Conv_IntToString` (`self.CDHeure`)) " : " (`KismetStringLibrary.Conv_IntToString` (`self.CDMinute`)) " : " (`KismetStringLibrary.Conv_IntToString` (`self.CDSecond`)))) (`self.Text3DComponent`)))

(fn `UserConstructionScript`)