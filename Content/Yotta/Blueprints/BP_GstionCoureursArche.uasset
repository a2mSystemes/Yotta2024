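; Manages up to two on-screen runner displays for a race arch, driven by DTFlux spotter and finisher events.
; Spotter events or E spawn BP_coureur1 in a free slot and slide it from PositionDepart to its position using timeline lerps.
; Arrivals update rank and time, wait, then slide the actor back and destroy it.
; Names, arrival results and R-key bib checks are hard-coded test values, and finisher data is unused.
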(event `Key|E`
  (params (Key :type "Key Structure"))
  ;[1 1 1] Spotter
  (:`Pressed`
    (if (`self.Coureur1`) :!label _label
      (if (not (`self.Coureur2`))
        (bind _bib (break `DTFluxSplitRanking` (stale `SpotterDetected` SpotterData)))
        (`self.ApparitionCoureur2` _bib "T.Henry" 2))
      (else
        (`self.ApparitionCoureur1` _bib "F. Biden" 2)))))

(event `self.ReceiveBeginPlay`
  (bind _returnvalue (subsystem `DTFluxSubsystem`))
  (add `DTFluxSubsystem.OnSpotter` _returnvalue (delegate `SpotterDetected`))
  (add `DTFluxSubsystem.OnFinisher` _returnvalue (delegate `FinisherDetected`)))

(event `SpotterDetected`
  (params (SpotterData :type "DTFluxSplitRanking Structure"))
  ;[1 1 1] Spotter
  (goto _label))

(event `Key|R`
  (params (Key :type "Key Structure"))
  ;[1 1 1] Finisher/Donne un bib
  (:`Pressed`
    (if (and (== 15 (`self.Bib1`)) (== true (`self.Coureur1`)))
      (`self.ArriveeCoureur1` 15 2 "17:26:30" :!label _label_2))
    (if (and (== 12 (`self.Bib2`)) (== true (`self.Coureur2`)))
      (`self.ArriveeCoureur2` 12 3 "17:26:34"))
    (if (== 0 (`self.Bib3`))
      _
      (elif (== 0 (`self.Bib4`))
        _))))

(event `FinisherDetected`
  (params (FinisherData :type "DTFluxSplitRanking Structure"))
  ;[1 1 1] Finisher/Donne un bib
  (goto _label_2))

(event `ArriveeCoureur1`
  (params (Bib :type Integer) (Rank :type Integer) (Time :type String))
  (bind _coureur1actor (`self.Coureur1Actor`))
  (bind _position1_location (`KismetMathLibrary.BreakTransform` (`self.Position1`)))
  (bind _position_depart_location (`KismetMathLibrary.BreakTransform` (`self.Position depart`)))
  ;[1 1 1] Arivée coureur 1
  (`/Game/Yotta/Blueprints/BP_coureur1.Change Rank Time Coureur` _coureur1actor Bib Rank Time)
  (`KismetSystemLibrary.Delay` (`self.Tempsaffichage`))
  (bind (_direction `_deplacement_vers_arrivée`) (`Timeline|Timeline_0` :!via `PlayFromStart`)
    (:`Update`
      (`self.K2_SetActorLocation` _coureur1actor (+ (* _position1_location (- (1.0 1.0 1.0) `_deplacement_vers_arrivée`)) (* `_deplacement_vers_arrivée` _position_depart_location)) false false))
    (:`Finished`
      (`self.K2_DestroyActor` _coureur1actor)
      (set `self.Coureur1` false))))

(event `ApparitionCoureur1`
  (params (Bib :type Integer) (Name :type String) (Contest :type Integer))
  (bind _position1_location (`KismetMathLibrary.BreakTransform` (`self.Position1`)))
  (bind _position_depart_location (`KismetMathLibrary.BreakTransform` (`self.Position depart`)))
  (bind _bib1 (`self.Bib1`))
  ;[1 1 1] Animation coureur1
  (set `self.Coureur1` true)
  (set `self.Bib1` Bib)
  (bind _returnvalue (`|SpawnActorFromClass` "/Game/Yotta/Blueprints/BP_coureur1.BP_coureur1_C" (`self.Position depart`) "Undefined" "MultiplyWithRoot" null null))
  (bind _output_get (set `self.Coureur1Actor` _returnvalue))
  (`/Game/Yotta/Blueprints/BP_coureur1.ChangeInfosCoureur` _output_get _bib1 Name)
  (`/Game/Yotta/Blueprints/BP_coureur1.Change Rank Time Coureur` _output_get _bib1 0 "-")
  (`/Game/Yotta/Blueprints/BP_coureur1.ChangePhotoCoureur1` _output_get _bib1 Contest)
  (bind (_direction `_deplacement_vers_arrivée`) (`Timeline|Timeline` :!via `PlayFromStart`)
    (:`Update`
      (`self.K2_SetActorLocation` _output_get (+ (* _position_depart_location (- (1.0 1.0 1.0) `_deplacement_vers_arrivée`)) (* `_deplacement_vers_arrivée` _position1_location)) false false))))

(event `ArriveeCoureur2`
  (params (Bib :type Integer) (Rank :type Integer) (Time :type String))
  (bind _position_depart_location (`KismetMathLibrary.BreakTransform` (`self.Position depart`)))
  (bind _coureur2actor (`self.Coureur2Actor`))
  (bind _position2_location (`KismetMathLibrary.BreakTransform` (`self.Position2`)))
  ;[1 1 1] Arivée coureur 1
  (`/Game/Yotta/Blueprints/BP_coureur1.Change Rank Time Coureur` _coureur2actor Bib Rank Time)
  (`KismetSystemLibrary.Delay` (`self.Tempsaffichage`))
  (bind (_direction `_deplacement_vers_arrivée`) (`Timeline|Timeline_2` :!via `PlayFromStart`)
    (:`Update`
      (`self.K2_SetActorLocation` _coureur2actor (+ (* _position2_location (- (1.0 1.0 1.0) `_deplacement_vers_arrivée`)) (* `_deplacement_vers_arrivée` _position_depart_location)) false false))
    (:`Finished`
      (`self.K2_DestroyActor` _coureur2actor)
      (set `self.Coureur2` false))))

(event `ApparitionCoureur2`
  (params (Bib :type Integer) (Name :type String) (Contest :type Integer))
  (bind _bib2 (`self.Bib2`))
  (bind _position2_location (`KismetMathLibrary.BreakTransform` (`self.Position2`)))
  (bind _position_depart_location (`KismetMathLibrary.BreakTransform` (`self.Position depart`)))
  ;[1 1 1] Animation coureur1
  (set `self.Coureur2` true)
  (set `self.Bib2` Bib)
  (bind _returnvalue (`|SpawnActorFromClass` "/Game/Yotta/Blueprints/BP_coureur1.BP_coureur1_C" (`self.Position depart`) "Undefined" "MultiplyWithRoot" null null))
  (bind _output_get (set `self.Coureur2Actor` _returnvalue))
  (`/Game/Yotta/Blueprints/BP_coureur1.ChangeInfosCoureur` _output_get _bib2 Name)
  (`/Game/Yotta/Blueprints/BP_coureur1.Change Rank Time Coureur` _output_get _bib2 0 "-test")
  (`/Game/Yotta/Blueprints/BP_coureur1.ChangePhotoCoureur1` _output_get _bib2 Contest)
  (bind (_direction `_deplacement_vers_arrivée`) (`Timeline|Timeline_1` :!via `PlayFromStart`)
    (:`Update`
      (`self.K2_SetActorLocation` _output_get (+ (* _position_depart_location (- (1.0 1.0 1.0) `_deplacement_vers_arrivée`)) (* `_deplacement_vers_arrivée` _position2_location)) false false))))

(fn `Set Values Coureur`
  (params (Bib :type Integer) (Contest :type Integer) (Split :type Integer) (Name :type String) (Time :type String) (Rank :type Integer)))

(fn `UserConstructionScript`)