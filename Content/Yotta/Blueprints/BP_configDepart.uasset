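; Start-display controller for the Yotta 2024 race, building a pursuit start board and setting contest and stage signage.
; On BeginPlay it refreshes DTFlux rankings for a hardcoded contest and stage, then fetches pursuit start times.
; Each runner gets a BP_LignePoursuite row, offset vertically by index and filled with bib and start time.
; Separate functions set the 3D stage title and load contest logos from absolute disk paths into a dynamic material.
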(event `self.ReceiveBeginPlay`
  (bind _tableaucoureurs (`self.Get Tableau Coureurs Triés` 5 (`|MakeArray` 2) 6000.0))
  (`self.CreateTableauDepart` _tableaucoureurs))

(fn `Change Contest Name`
  (params (Contest :type Integer))
  (switch `int` Contest
    (:`1`
      ;[1 1 1] Yotta XPS
      (set `self.Filenamedepart` "E:/Yotta2024 Unreal/Yotta2024/Content/Yotta/Medias/24-STREAM-MEDIAS/ContestYottaxps.png" :!label _label))
    (:`2`
      ;[1 1 1] Yotta XP elite
      (set `self.Filenamedepart` "E:/Yotta2024 Unreal/Yotta2024/Content/Yotta/Medias/24-STREAM-MEDIAS/ContestYottaxpelite.png" :!label _label_2))
    (:`3`
      (goto _label_2))
    (:`4`
      ;[1 1 1] Yotta XP
      (set `self.Filenamedepart` "E:/Yotta2024 Unreal/Yotta2024/Content/Yotta/Medias/24-STREAM-MEDIAS/ContestYottaxp.png" :!label _label_3))
    (:`5`
      (goto _label_3))
    (:`6`
      (goto _label))
    (:`10`
      ;[1 1 1] Yotta XPS relais
      (set `self.Filenamedepart` "E:/Yotta2024 Unreal/Yotta2024/Content/Yotta/Medias/24-STREAM-MEDIAS/ContestYottaxpsrelais.png")))
  (bind _returnvalue (`KismetRenderingLibrary.ImportFileAsTexture2D` (`self.Filenamedepart`)))
  (bind _returnvalue_2 (`PrimitiveComponent.CreateDynamicMaterialInstance` (`StaticMeshActor.StaticMeshComponent` (`self.ContestnameDepartObject`)) 0 "/Game/Yotta/Material/Arche/M_Arche_Contest.M_Arche_Contest" "None"))
  (`MaterialInstanceDynamic.SetTextureParameterValue` _returnvalue_2 "Contest_texture" _returnvalue))

(fn `Change Stage Et Contest Name`
  (params (Contest :type Integer) (Stage :type Integer))
  (bind _stagenamevar (`self.StageNameVar`))
  (bind _output_get (set `self.ContestDepartID` Contest))
  (set `self.StageDepartID` Stage)
  (`self.Change Contest Name` _output_get)
  ;[1 1 1] clear variable
  (set `self.StageNameVar` "")
  ;[1 1 1] Nommer étape
  (switch `int` (`self.StageDepartID`)
    (:`Default`
      (set `self.StageNameVar` ""))
    (:`1`
      (set `self.StageNameVar` "kilo")
      ;[1 1 1] Nommer course
      (switch `int` (`self.ContestDepartID`) :!label _label
        (:`1`
          (set `self.StageNameVar` (`KismetStringLibrary.Concat_StrStr` _stagenamevar " XPS") :!label _label_2))
        (:`2`
          (set `self.StageNameVar` (`KismetStringLibrary.Concat_StrStr` _stagenamevar " XP") :!label _label_3))
        (:`3`
          (goto _label_3))
        (:`4`
          (goto _label_3))
        (:`5`
          (goto _label_3))
        (:`6`
          (goto _label_2))
        (:`10`
          (goto _label_2))))
    (:`2`
      (set `self.StageNameVar` "mega")
      (goto _label))
    (:`3`
      (set `self.StageNameVar` "giga")
      (goto _label))
    (:`4`
      (set `self.StageNameVar` "tera")
      (goto _label))
    (:`5`
      (set `self.StageNameVar` "peta")
      (goto _label)))
  (set `Text3DComponent.Text` (`KismetTextLibrary.Conv_StringToText` _stagenamevar) (`AvaTextActor.Text3DComponent` (`self.StageNameDepartObject`))))

(fn `CreateTableauDepart`
  (params (TableauCoureurs :type "Array of DTFluxStageRanking Structure"))
  (bind _origine (`self.Origine`))
  (for (_array_element _array_index) TableauCoureurs
    (bind _returnvalue (`|SpawnActorFromClass` "/Game/Yotta/Blueprints/BP_LignePoursuite.BP_LignePoursuite_C" (`KismetMathLibrary.MakeTransform` (`KismetMathLibrary.MakeVector` (.x (.location _origine)) (.y (.location _origine)) (+ (* _array_index (`self.DecalageZLigne`)) (.z (.location _origine)))) (.rotation _origine) (.scale _origine)) "Undefined" "MultiplyWithRoot" self null))
    (bind (_bib _rank _gap _timeswim _timetransition _timerun _timestart) (break `DTFluxStageRanking` _array_element))
    (`/Game/Yotta/Blueprints/BP_LignePoursuite.SetValues` _returnvalue _bib _timestart)
    (bind (_year _month _day _hour _minute _second) (`KismetMathLibrary.BreakDateTime` _timestart))
    (`KismetSystemLibrary.PrintString` (`KismetStringLibrary.Concat_StrStr` (`KismetStringLibrary.Conv_IntToString` _hour) "h" (`KismetStringLibrary.Conv_IntToString` _minute) "m" (`KismetStringLibrary.Conv_IntToString` _second) "s"))))

(fn `Get Tableau Coureurs Triés`
  (params (Stage :type Integer) (Contest :type "Array of Integer") (DeltaTimeSecondes :type "Float (double-precision)"))
  (returns (TableauCoureurs :type "Array of DTFluxStageRanking Structure"))
  (bind _returnvalue (subsystem `DTFluxSubsystem`))
  (for _array_element Contest
    (`DTFluxSubsystem.UpdateStageRanking` _returnvalue _array_element Stage -1))
  (bind _returnvalue_2 (`DTFluxSubsystem.GetDataStorage` _returnvalue))
  (bind _returnvalue_3 (`DTFluxDataStorage.GetPoursuitWithTimeStart` _returnvalue_2 Contest Stage DeltaTimeSecondes))
  (return _returnvalue_3))

(fn `UserConstructionScript`)