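; Actor for one row of a contest stage results table, showing a competitor's timing in a swim, transition and run race.
; SetValuesLigneTableau converts its inputs to text and writes bib, name, total time, gap and the three split times into the row's text fields.
; The Rank field always shows zero because the Rank input is not used.
; The event graph and construction script contain no logic.
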(fn `SetValuesLigneTableau`
  (params (bib :type Integer) (Rank :type Integer) (Name :type String) (Time :type String) (Gap :type String) (TimeSwim :type String) (TimeTransition :type String) (TimeRun :type String))
  (set `Text3DComponent.Text` (`KismetTextLibrary.Conv_IntToText` bib) (`self.Bib`))
  (set `Text3DComponent.Text` (`KismetTextLibrary.Conv_IntToText` 0) (`self.Rank`))
  (set `Text3DComponent.Text` (`KismetTextLibrary.Conv_StringToText` Name) (`self.Nom concat`))
  (set `Text3DComponent.Text` (`KismetTextLibrary.Conv_StringToText` Time) (`self.Time`))
  (set `Text3DComponent.Text` (`KismetTextLibrary.Conv_StringToText` Gap) (`self.Gap`))
  (set `Text3DComponent.Text` (`KismetTextLibrary.Conv_StringToText` TimeSwim) (`self.TimeSwim`))
  (set `Text3DComponent.Text` (`KismetTextLibrary.Conv_StringToText` TimeTransition) (`self.TimeTransition`))
  (set `Text3DComponent.Text` (`KismetTextLibrary.Conv_StringToText` TimeRun) (`self.TimeRun`)))

(fn `UserConstructionScript`)