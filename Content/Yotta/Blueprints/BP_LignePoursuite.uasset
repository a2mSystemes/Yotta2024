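; BP_LignePoursuite is one line of a pursuit start display, showing a competitor's bib and name.
; SetValues fills both texts and spawns an owned BP_Counter_Child_Poursuite at the DecalageChrono offset, then starts it with the given start time, bib and "GO" end text.
; WantedToRemove forwards a bib's removal request to the owning BP_configDepart.
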(fn `SetIndex`
  (params (Index :type Integer))
  (set `self.Index` Index))

(fn `SetValues`
  (params (Bib :type Integer) (timeStart :type "DateTime Structure") (Name :type String))
  (bind (_decalagechrono_location _decalagechrono_rotation _decalagechrono_scale) (`KismetMathLibrary.BreakTransform` (`self.DecalageChrono`)))
  (bind (_returnvalue_location _returnvalue_rotation _returnvalue_scale) (`KismetMathLibrary.BreakTransform` (`self.GetTransform` self)))
  (set `Text3DComponent.Text` (`KismetTextLibrary.Conv_IntToText` Bib) (`self.Bib`))
  (set `Text3DComponent.Text` (`KismetTextLibrary.Conv_StringToText` Name) (`self.Nom`))
  (bind _returnvalue (`|SpawnActorFromClass` "/Game/Yotta/Blueprints/BP_Counter_Child_Poursuite.BP_Counter_Child_Poursuite_C" (`KismetMathLibrary.MakeTransform` (+ _returnvalue_location _decalagechrono_location) (struct) (* _returnvalue_scale _decalagechrono_scale)) "Undefined" "MultiplyWithRoot" self null))
  (`/Game/Yotta/Blueprints/BP_Counter.SetTimerType` _returnvalue -1 "GO" "/Game/Yotta/Material/M_Blanc.M_Blanc")
  (`/Game/Yotta/Blueprints/BP_Counter_Child_Poursuite.SetTimerTimeAndStart` _returnvalue timeStart)
  (`/Game/Yotta/Blueprints/BP_Counter_Child_Poursuite.Set bib` _returnvalue Bib))

(fn `UserConstructionScript`)

(fn `Wanted to remove`
  (params (bib :type Integer))
  (bind _asbp_config_depart (cast `/Game/Yotta/Blueprints/BP_configDepart` (`self.GetOwner`)))
  (`/Game/Yotta/Blueprints/BP_configDepart.RemoveMe` _asbp_config_depart bib)
  (return))