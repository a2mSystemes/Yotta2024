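; BP_ListeStream builds a vertical list of runner rows showing name, rank and bib, apparently a race standings display.
; At BeginPlay, ConstruireAVA spawns a BP_LigneListe for each TableauCoureur entry, fills it and stacks it by DeltaRowZ from the actor's location.
; A timer then fires a hardcoded swap of the third and fourth rows through their spline movement, which looks like a reordering test.
; UpdateLine is an empty stub.
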(event `self.ReceiveBeginPlay`
  (`self.ConstruireAVA`)
  (`KismetSystemLibrary.K2_SetTimerDelegate` (delegate `CustomEvent`) 2.0))

(event `CustomEvent`
  (bind _tableaucoureurs (`self.TableauCoureurs`))
  (bind _output (`|GetArrayItem` _tableaucoureurs 3))
  (bind _output_2 (`|GetArrayItem` _tableaucoureurs 2))
  (`/Game/Yotta/Blueprints/BP_LigneListe.Set Spline Mouvement` _output (`self.K2_GetActorLocation` _output_2))
  (`/Game/Yotta/Blueprints/BP_LigneListe.MoveLine` _output)
  (`/Game/Yotta/Blueprints/BP_LigneListe.Set Spline Mouvement` _output_2 (`self.K2_GetActorLocation` _output))
  (`/Game/Yotta/Blueprints/BP_LigneListe.MoveLine` _output_2))

(fn `ConstruireAVA`
  (for _array_element (`self.TableauCoureur`)
    (`self.CreateLine` _array_element)))

(fn `CreateLine`
  (params (InLigne :type "/Game/Yotta/Temp_structure/ST_Tableau_Coureurs Structure"))
  (bind (_rank _name _bib) (break `/Game/Yotta/Temp_structure/ST_Tableau_Coureurs` InLigne))
  (bind (_returnvalue_x _returnvalue_y _returnvalue_z) (`KismetMathLibrary.BreakVector` (`self.K2_GetActorLocation`)))
  (bind _tableaucoureurs (`self.TableauCoureurs`))
  (bind _returnvalue (`|SpawnActorFromClass` "/Game/Yotta/Blueprints/BP_LigneListe.BP_LigneListe_C" (`KismetMathLibrary.MakeTransform` (0.0 0.0 0.0)) "Undefined" "MultiplyWithRoot" self null))
  (bind _returnvalue_2 (`KismetArrayLibrary.Array_Add` _tableaucoureurs _returnvalue))
  (bind _returnvalue_3 (+ (* _returnvalue_2 (`self.DeltaRowZ`)) _returnvalue_z))
  (`/Game/Yotta/Blueprints/BP_LigneListe.Set Values Line` _returnvalue _name _rank _bib _returnvalue_3)
  (`SceneComponent.K2_SetRelativeTransform` (`Actor.RootComponent` (`|GetArrayItem` _tableaucoureurs _returnvalue_2)) (`KismetMathLibrary.MakeTransform` (`KismetMathLibrary.MakeVector` _returnvalue_x _returnvalue_y _returnvalue_3)) false false))

(fn `UpdateLine`
  (params (InLigne :type "/Game/Yotta/Temp_structure/ST_Tableau_Coureurs Structure")))

(fn `UserConstructionScript`)