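; Runner display actor that shows one race competitor's photo, name, bib, rank and time.
; Its functions update the text fields, with a zero rank blanking the rank and leaving the time untouched.
; The photo is loaded at runtime from a hardcoded disk folder by bib number, falling back to a relay or solo silhouette by contest ID.
; The imported texture feeds a dynamic material instance on the photo component.
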(event `self.ReceiveBeginPlay`)

(fn `Change Rank Time Coureur`
  (params (Bib :type Integer) (Rank :type Integer) (Time :type String))
  (if (== Rank 0)
    (set `Text3DComponent.Text` " " (`self.Rank1`))
    (else
      (set `Text3DComponent.Text` (`KismetTextLibrary.Conv_IntToText` Rank) (`self.Rank1`))
      (set `Text3DComponent.Text` (`KismetTextLibrary.Conv_StringToText` Time) (`self.Time1`)))))

(fn `ChangeInfosCoureur`
  (params (Bib :type Integer) (Name :type String))
  (set `Text3DComponent.Text` (`KismetTextLibrary.Conv_StringToText` Name) (`self.Name1`))
  (set `Text3DComponent.Text` (`KismetTextLibrary.Conv_IntToText` Bib) (`self.Bib1`)))

(fn `ChangePhotoCoureur1`
  (params (Bib :type Integer) (ContestID :type Integer))
  (bind _returnvalue (`KismetStringLibrary.Concat_StrStr` "E:/YottaPhotoCoureurs/" (`KismetStringLibrary.Conv_IntToString` Bib) ".png"))
  ;[1 1 1] Vérifie si le fichier existe
  (bind _returnvalue_2 (`BlueprintFileUtilsBPLibrary.FileExists` _returnvalue))
  (if _returnvalue_2
    (set `self.FileNamePhoto` _returnvalue)
    (else
      ;[1 1 1] Affiche les silouhettes si le fichier n'existe pas
      (`KismetSystemLibrary.PrintString` "File dosent exist")
      (if (== ContestID 10)
        (set `self.FileNamePhoto` "E:/YottaPhotoCoureurs/24-ARCHE-JoueursMysteresRelais.png")
        (else
          (set `self.FileNamePhoto` "E:/YottaPhotoCoureurs/24-ARCHE-JoueursMysteresSolo.png")))))
  ;[1 1 1] Importe le fichier en tant que texture
  (bind _returnvalue_3 (`KismetRenderingLibrary.ImportFileAsTexture2D` (`self.FileNamePhoto`)))
  (bind _returnvalue_4 (`PrimitiveComponent.CreateDynamicMaterialInstance` (`self.PhotoCoureur1`) 0 "/Game/Yotta/Material/Arche/M_coureur1.M_coureur1" "None"))
  (`MaterialInstanceDynamic.SetTextureParameterValue` _returnvalue_4 "Coureur1texture" _returnvalue_3))

(fn `NewFunction`)

(fn `UserConstructionScript`)