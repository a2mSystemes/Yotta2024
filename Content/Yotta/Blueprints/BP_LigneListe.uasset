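; Leaderboard line actor showing one competitor's rank, bib and name, truncating long names with "..." and giving first place a distinct rank background.
; Tick places it at its owner's location plus a height offset.
; MoveLine animates rank changes with a timeline along a runtime-built spline that detours sideways, currently using a hardcoded vertical move.
; BeginPlay only prints a DTFlux subsystem name lookup for a hardcoded bib as debug.
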(event `self.ReceiveBeginPlay`
  (bind _returnvalue (`DTFluxSubsystem.GetDataStorage` (subsystem `DTFluxSubsystem`)))
  (bind _returnvalue_2 (`DTFluxDataStorage.GetConcurrentFormatedName` _returnvalue 759 true 5))
  (`KismetSystemLibrary.PrintString` _returnvalue_2 true true (struct :`G` 0.66 :`B` 1.0 :`A` 1.0) 10.0))

(event `self.ReceiveTick`
  (params (DeltaSeconds :type "Float (single-precision)"))
  (bind _returnvalue (`self.K2_GetActorLocation` (`self.GetOwner`)))
  (bind _returnvalue_2 (+ _returnvalue (`KismetMathLibrary.MakeVector` 0.0 0.0 (`self.Zposition`))))
  (if (!= (`self.CurrentParentLocation`) _returnvalue)
    (`self.K2_SetActorLocation` _returnvalue_2)
    (set `self.CurrentParentLocation` _returnvalue_2)))

(event `MoveLine`
  (bind _splinechgtrank (`self.SplineChgtRank`))
  (`self.Move To` (0.0 0.0 200.0))
  (`TimelineComponent.SetPlayRate` (`self.MoveTimeline`) (/ 1.0 (`self.TempsAnimation`)))
  (bind (_direction _newtrack_0) (`Timeline|MoveTimeline` :!via `PlayFromStart`)
    (:`Update`
      (`self.K2_SetActorTransform` (`KismetMathLibrary.MakeTransform` (`SplineComponent.GetLocationAtDistanceAlongSpline` _splinechgtrank (`KismetMathLibrary.Lerp` 0.0 (`SplineComponent.GetSplineLength` _splinechgtrank) _newtrack_0) "Local"))))))

(fn `Move To`
  (params (NewLocation :type "Vector Structure"))
  (locals (NewLocalVar :type "Array of Vector Structure"))
  (`self.Set Spline Mouvement` NewLocation))

(fn `Set Spline Mouvement`
  (params (Target :type "Vector Structure"))
  (locals (SplinePoints :type "Array of Vector Structure"))
  (bind _returnvalue (`self.K2_GetActorLocation`))
  (bind _splinepoints (`local.SplinePoints`))
  (bind _returnvalue_2 (+ _returnvalue (-100.0 0.0 0.0)))
  (bind _returnvalue_3 (+ _returnvalue_2 (`KismetMathLibrary.MakeVector` 0.0 0.0 Target_Z)))
  (`SplineComponent.ClearSplinePoints` (`self.SplineChgtRank`) true)
  (`KismetArrayLibrary.Array_Clear` _splinepoints)
  (`KismetArrayLibrary.Array_Add` _splinepoints _returnvalue)
  (`KismetArrayLibrary.Array_Add` _splinepoints _returnvalue_2)
  (`KismetArrayLibrary.Array_Add` _splinepoints _returnvalue_3)
  (`KismetArrayLibrary.Array_Add` _splinepoints (+ _returnvalue_3 (100.0 0.0 0.0)))
  (`SplineComponent.SetSplinePoints` (`self.SplineChgtRank`) _splinepoints "Local" true)
  (return))

(fn `Set Values Line`
  (params (Nom :type String) (Rank :type Integer) (Bib :type Integer) (Zposition :type "Float (double-precision)"))
  (`self.SetBibYotta` Bib)
  (`self.SetRankYotta` Rank)
  (`self.SetNameYotta` Nom)
  (set `self.Zposition` Zposition)
  (return))

(fn `SetBibYotta`
  (params (Bib :type Integer))
  (set `Text3DComponent.Text` (`KismetTextLibrary.Conv_IntToText` Bib) (`self.Bib`)))

(fn `SetNameYotta`
  (params (Nom :type String))
  (bind _name (`self.Name`))
  ;[0.4048 1 0.2977] Détermine la longueur du nom et décide si ça passe
  (if (<= (`KismetStringLibrary.Len` Nom) (`self.MaxCaractereNom`))
    (set `Text3DComponent.Text` (`KismetTextLibrary.Conv_StringToText` Nom) _name)
    (else
      (set `Text3DComponent.Text` (`KismetTextLibrary.Conv_StringToText` (`KismetStringLibrary.Concat_StrStr` (`KismetStringLibrary.Left` Nom (- (`self.MaxCaractereNom`) 3)) "...")) _name))))

(fn `SetRankYotta`
  (params (Rank :type Integer))
  (bind _fondrank (`self.FondRank`))
  (set `Text3DComponent.Text` (`KismetTextLibrary.Conv_IntToText` Rank) (`self.Rank`))
  ;[1 1 1] Choisi l'icone à mettre derrière le numéro (icône rouge si premier, noir sinon)
  (if (== Rank 1)
    (`PrimitiveComponent.SetMaterial` _fondrank 0 "/Game/Yotta/Material/M_FondRank1er.M_FondRank1er")
    (else
      (`PrimitiveComponent.SetMaterial` _fondrank 0 "/Game/Yotta/Material/M_FondRank.M_FondRank"))))

(fn `UserConstructionScript`)