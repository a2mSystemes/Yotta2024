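; BP_YottaText is an actor that displays one ranking line: a name, a rank and a bib number.
; SetValuesLine fills all three texts through dedicated setters, shortening names over MaxCaractereNom with a trailing "...".
; The rank setter also swaps the material behind the number to highlight first place.
; BeginPlay, overlap, Tick and the construction script are empty, so updates rely on calls to these functions.
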(event `self.ReceiveTick`
  (params (DeltaSeconds :type "Float (single-precision)")))

(fn `SetBibYotta`
  (params (Bib :type Integer))
  (set `Text3DComponent.Text` (`KismetTextLibrary.Conv_IntToText` Bib) (`self.Bib`)))

(fn `SetNameYotta`
  (params (Nom :type String))
  (bind _name (`self.Name`))
  ;[0.4048 1 0.2977] Détermine la longueur du nom et décide si ça passe
  (if (<= (`KismetStringLibrary.Len` Nom) (`self.MaxCaractereNom`))
    (set `Text3DComponent.Text` (`KismetTextLibrary.Conv_StringToText` Nom) _name)
    (else
      (set `Text3DComponent.Text` (`KismetTextLibrary.Conv_StringToText` (`KismetStringLibrary.Concat_StrStr` (`KismetStringLibrary.Left` Nom (- (`self.MaxCaractereNom`) 3)) "...")) _name))))

(fn `SetRankYotta`
  (params (Rank :type Integer))
  (bind _fondrank (`self.FondRank`))
  (set `Text3DComponent.Text` (`KismetTextLibrary.Conv_IntToText` Rank) (`self.Rank`))
  ;[1 1 1] Choisi l'icone à mettre derrière le numéro (icône rouge si premier, noir sinon)
  (if (== Rank 1)
    (`PrimitiveComponent.SetMaterial` _fondrank 0 "/Game/Yotta/Material/M_FondRank1er.M_FondRank1er")
    (else
      (`PrimitiveComponent.SetMaterial` _fondrank 0 "/Game/Yotta/Material/M_FondRank.M_FondRank"))))

(fn `SetValuesLine`
  (params (Nom :type String) (Rank :type Integer) (Bib :type Integer))
  (`self.SetBibYotta` Bib)
  (`self.SetRankYotta` Rank)
  (`self.SetNameYotta` Nom)
  (return))

(fn `UserConstructionScript`)