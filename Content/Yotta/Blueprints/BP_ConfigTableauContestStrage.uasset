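; Leaderboard actor that builds a top-10 stage ranking board for a timed swim/run race from DTFlux data.
; On BeginPlay it requests a ranking update for the current contest and stage, then after 0.5 s reads stored rankings for hardcoded contest 2, stage 2.
; It spawns one BP_LigneTableauContestStage row per entry, offset in Y/Z from OrigineTableau, filled with bib, rank, truncated name, times, gap and shortened splits.
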(event `self.ReceiveBeginPlay`
  (bind _returnvalue (subsystem `DTFluxSubsystem`))
  (`DTFluxSubsystem.UpdateStageRanking` _returnvalue (`self.CurrentContest`) (`self.CurrentStage`) -1)
  (`KismetSystemLibrary.Delay` 0.5)
  (`self.LignesTableauStage` 2 2 (`self.OrigineTableau`) (`self.Delta Z`) (`self.Delta Y`) _returnvalue))

(fn `LignesTableauStage`
  (params (Contest :type Integer) (Stage :type Integer) (Origine :type "Transform Structure") (DeltaZ :type "Float (double-precision)") (DeltaY :type "Float (double-precision)") (Subsystem :type "DTFluxSubsystem Object Reference"))
  (bind _returnvalue (`DTFluxSubsystem.GetDataStorage` Subsystem))
  (bind _returnvalue_2 (`DTFluxDataStorage.GetStageRanking` _returnvalue Contest Stage))
  (if (`KismetArrayLibrary.Array_IsNotEmpty` _returnvalue_2)
    (for (_array_element _array_index) _returnvalue_2
      (if (>= _array_index 10)
        (break)
        (else
          (bind _returnvalue_3 (`|SpawnActorFromClass` "/Game/Yotta/Blueprints/BP_LigneTableauContestStage.BP_LigneTableauContestStage_C" (`KismetMathLibrary.MakeTransform` (+ (.location Origine) (`KismetMathLibrary.MakeVector` 0.0 (* _array_index DeltaY) (* _array_index DeltaZ))) (.rotation Origine) (.scale Origine)) "Undefined" "MultiplyWithRoot" null null))
          (bind (_bib _rank _gap _time _timeswim _timetransition _timerun) (break `DTFluxStageRanking` _array_element))
          (bind _returnvalue_4 (`DTFluxModelHelper.GetParticipantString` _bib true 15))
          (`/Game/Yotta/Blueprints/BP_LigneTableauContestStage.SetValuesLigneTableau` _returnvalue_3 _bib _rank _returnvalue_4 _time _gap (`KismetStringLibrary.Right` _timeswim 5) (`KismetStringLibrary.Right` _timetransition 5) (`KismetStringLibrary.Right` _timerun 5)))))))

(fn `UserConstructionScript`)