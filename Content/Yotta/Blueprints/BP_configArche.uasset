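; BP_configArche configures the race arch display for the Yotta event, showing the current contest banner and stage name.
; On BeginPlay it passes ContestID and StageID to ChangeStageEtContestName, which builds the 3D stage text from a metric-prefix name plus an XP or XPS suffix.
; ChangeContestName imports a contest PNG from hardcoded absolute E: drive paths into a dynamic material on the banner mesh.
; StatutStageWaiting and MediaPlateStart are empty stubs.
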(event `self.ReceiveBeginPlay`
  (`self.Change Stage Et Contest Name` (`self.ContestID`) (`self.StageID`)))

(fn `Change Contest Name`
  (params (Contest :type Integer))
  (switch `int` Contest
    (:`1`
      ;[1 1 1] Yotta XPS
      (set `self.Filename` "E:/Yotta2024 Unreal/Yotta2024/Content/Yotta/Medias/24-STREAM-MEDIAS/ContestYottaxps.png" :!label _label))
    (:`2`
      ;[1 1 1] Yotta XP elite
      (set `self.Filename` "E:/Yotta2024 Unreal/Yotta2024/Content/Yotta/Medias/24-STREAM-MEDIAS/ContestYottaxpelite.png" :!label _label_2))
    (:`3`
      (goto _label_2))
    (:`4`
      ;[1 1 1] Yotta XP
      (set `self.Filename` "E:/Yotta2024 Unreal/Yotta2024/Content/Yotta/Medias/24-STREAM-MEDIAS/ContestYottaxp.png" :!label _label_3))
    (:`5`
      (goto _label_3))
    (:`6`
      (goto _label))
    (:`10`
      ;[1 1 1] Yotta XPS relais
      (set `self.Filename` "E:/Yotta2024 Unreal/Yotta2024/Content/Yotta/Medias/24-STREAM-MEDIAS/ContestYottaxpsrelais.png")))
  (bind _returnvalue (`KismetRenderingLibrary.ImportFileAsTexture2D` (`self.Filename`)))
  (bind _returnvalue_2 (`PrimitiveComponent.CreateDynamicMaterialInstance` (`StaticMeshActor.StaticMeshComponent` (`|ConvertAsset` (`self.ContestNameObject`))) 0 "/Game/Yotta/Material/Arche/M_Arche_Contest.M_Arche_Contest" "None"))
  (`MaterialInstanceDynamic.SetTextureParameterValue` _returnvalue_2 "Contest_texture" _returnvalue))

(fn `Change Stage Et Contest Name`
  (params (Contest :type Integer) (Stage :type Integer))
  (bind _stagenamevar (`self.StageNameVar`))
  (bind _output_get (set `self.ContestID` Contest))
  (set `self.StageID` Stage)
  (`self.Change Contest Name` _output_get)
  ;[1 1 1] clear variable
  (set `self.StageNameVar` "")
  ;[1 1 1] Nommer étape
  (switch `int` (`self.StageID`)
    (:`Default`
      (set `self.StageNameVar` ""))
    (:`1`
      (set `self.StageNameVar` "kilo")
      ;[1 1 1] Nommer course
      (switch `int` (`self.ContestID`) :!label _label
        (:`1`
          (set `self.StageNameVar` (`KismetStringLibrary.Concat_StrStr` _stagenamevar " XPS") :!label _label_2))
        (:`2`
          (set `self.StageNameVar` (`KismetStringLibrary.Concat_StrStr` _stagenamevar " XP") :!label _label_3))
        (:`3`
          (goto _label_3))
        (:`4`
          (goto _label_3))
        (:`5`
          (goto _label_3))
        (:`6`
          (goto _label_2))
        (:`10`
          (goto _label_2))))
    (:`2`
      (set `self.StageNameVar` "mega")
      (goto _label))
    (:`3`
      (set `self.StageNameVar` "giga")
      (goto _label))
    (:`4`
      (set `self.StageNameVar` "tera")
      (goto _label))
    (:`5`
      (set `self.StageNameVar` "peta")
      (goto _label)))
  (set `Text3DComponent.Text` (`KismetTextLibrary.Conv_StringToText` _stagenamevar) (`AvaTextActor.Text3DComponent` (`|ConvertAsset` (`self.StageNameObject`)))))

(fn `MediaPlateStart`)

(fn `Statut Stage Waiting`)

(fn `UserConstructionScript`)