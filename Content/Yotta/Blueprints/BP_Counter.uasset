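; BP_Counter is an on-screen clock that shows hh:mm:ss text for contest stages, counting by a configurable step with a set material.
; SetTimerContestStage seeds it from DTFlux stage data: time left to cutoff for StageId below 5, otherwise time since start.
; SetGoTime displays a scheduled start time and polls until it passes, then starts counting.
; A looping one-second timer updates the text, showing the end text and stopping below one.
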(event `self.ReceiveBeginPlay`)

(fn `Create Timer`
  (bind _returnvalue (`KismetSystemLibrary.K2_SetTimer` null "Update" 1.0 true false -1.0))
  (set `self.TimerRef` _returnvalue))

(fn `GetTimeString`
  (params (Time :type "DateTime Structure"))
  (returns (TimeText :type Text))
  (return (`|FormatText` "{hh}:{mm}:{ss}" (`KismetTextLibrary.Conv_IntToText` Time_Hour false false 2) (`KismetTextLibrary.Conv_IntToText` Time_Minute false false 2) (`KismetTextLibrary.Conv_IntToText` Time_Second false false 2))))

(fn `Set Go Time`
  (params (DelayMin :type Integer) (DelaySec :type Integer))
  (locals (NewLocalVar :type "TimerHandle Structure"))
  (bind _returnvalue (+ (`KismetMathLibrary.Now`) (`KismetMathLibrary.MakeTimespan` 0 0 DelayMin DelaySec)))
  (set `self.When` _returnvalue)
  (set `Text3DComponent.Text` (`|FormatText` "starting at {date}" (`self.GetTimeString` _returnvalue)) (`self.TextCounter`))
  (bind _returnvalue_2 (`KismetSystemLibrary.K2_SetTimer` null "watchStartTime" 0.2 true false 0.2))
  (set `self.WaitingTimer` _returnvalue_2)
  (return))

(fn `SetTimerContestStage`
  (params (ContestId :type Integer) (StageId :type Integer))
  (bind _returnvalue (`KismetMathLibrary.Now`))
  (bind _returnvalue_2 (`DTFluxSubsystem.GetDataStorage` (subsystem `DTFluxSubsystem`)))
  (bind (_outstage _returnvalue_3) (`DTFluxDataStorage.GetStage` _returnvalue_2 ContestId StageId))
  (if _returnvalue_3
    (if (< StageId 5)
      (bind (_id _name _starttime _endtime _cutoff) (break `DTFluxStage` _outstage))
      (set `self.TimeValue` (`KismetMathLibrary.FTrunc` (`KismetMathLibrary.GetTotalSeconds` (- _cutoff _returnvalue))))
      (else
        (set `self.TimeValue` (`KismetMathLibrary.FTrunc` (`KismetMathLibrary.GetTotalSeconds` (- _returnvalue _starttime))))))
    (`self.Create Timer`)))

(fn `SetTimerType`
  (params (Jump :type Integer) (EndText :type String) (Color :type "Material Object Reference"))
  (set `self.JumpType` Jump)
  (set `self.FinalTextType` EndText)
  (bind _output_get (set `self.Color` Color))
  (set `Text3DComponent.FrontMaterial` _output_get (`self.TextCounter`)))

(fn `Update`
  (`self.UpdateText` (`self.JumpType`) (`self.FinalTextType`))
  (return))

(fn `UpdateText`
  (params (Jump :type Integer) (FinalText :type String))
  (bind _timevalue (`self.TimeValue`))
  (bind _textcounter (`self.TextCounter`))
  (set `self.TimeValue` (+ (`self.TimeValue`) Jump))
  (if (< (`self.TimeValue`) 1)
    (set `Text3DComponent.Text` (`KismetTextLibrary.Conv_StringToText` FinalText) _textcounter)
    (`KismetSystemLibrary.K2_ClearAndInvalidateTimerHandle` (`self.TimerRef`))
    (else
      (set `Text3DComponent.Text` (`|FormatText` "{hh}:{mm}:{ss}" (`KismetTextLibrary.Conv_IntToText` (/ _timevalue 3600) false false 2) (`KismetTextLibrary.Conv_IntToText` (/ (mod _timevalue 3600) 60) false false 2) (`KismetTextLibrary.Conv_IntToText` (mod _timevalue 60) false false 2)) _textcounter)))
  (return))

(fn `UserConstructionScript`)

(fn `watchStartTime`
  (if (not (<= (`KismetMathLibrary.Now`) (`self.When`)))
    (`KismetSystemLibrary.K2_ClearAndInvalidateTimerHandle` (`self.WaitingTimer`))
    (`self.Create Timer`))
  (return))