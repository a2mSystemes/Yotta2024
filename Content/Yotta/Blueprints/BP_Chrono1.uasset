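; BP_Chrono1 is a countdown timer actor that shows its remaining time on a Text3D component.
; On BeginPlay it copies SetChrono1 into ElapsedTiming and starts a looping one-second timer.
; Each tick of that timer decrements the value and displays it as a timecode string trimmed to eight characters.
; The countdown has no stop or check at zero.
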(event `self.ReceiveBeginPlay`
  (set `self.ElapsedTiming` (`self.setChrono1`))
  (`KismetSystemLibrary.K2_SetTimerDelegate` (delegate `UpdateTimer`) 1.0 true))

(event `UpdateTimer`
  (bind _output_get (set `self.ElapsedTiming` (- (`self.ElapsedTiming`) 1)))
  (set `Text3DComponent.Text` (`KismetTextLibrary.Conv_StringToText` (`KismetStringLibrary.GetSubstring` (`TimeManagementBlueprintLibrary.Conv_TimecodeToString` (make `Timecode` 0 0 _output_get)) 0 8)) (`self.Text3DComponent`)))

(event `self.ReceiveTick`
  (params (DeltaSeconds :type "Float (single-precision)")))

(fn `UserConstructionScript`)