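; Synthe manager actor that can change an on-screen name held in a Motion Design (Avalanche) 3D text actor.
; ChangeNameSynthe finds AvaTextActors tagged "SynthNom", writes the given name into the first one's Text3D component, and logs whether one exists.
; BeginPlay separately calls EventTestMe with hard-coded time, contest and stage values; that event's body is not in these graphs.
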(event `self.ReceiveBeginPlay`
  (`self.EventTestMe` 12 1 2))

(fn `ChangeNameSynthe`
  (params (InNameSynthe :type String))
  (bind _outactors (`GameplayStatics.GetAllActorsOfClassWithTag` "/Script/AvalancheText.AvaTextActor" "SynthNom"))
  (if (>= (`KismetArrayLibrary.Array_Length` _outactors) 1)
    (`KismetSystemLibrary.PrintString` "ActorName Exist" false)
    (set `Text3DComponent.Text` (`KismetTextLibrary.Conv_StringToText` InNameSynthe) (`AvaTextActor.Text3DComponent` (`|GetArrayItem` _outactors)))
    (else
      (`KismetSystemLibrary.PrintString` "ActorName DoesNot Exist" false true (struct :`R` 1.0 :`G` 0.189016 :`B` 0.272736 :`A` 1.0))))
  (return))

(fn `UserConstructionScript`)