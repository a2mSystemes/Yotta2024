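; BP_Counter_Child_Poursuite is a counter child Blueprint, named for a pursuit, that counts from the time remaining until a given start time.
; SetTimerTimeAndStart converts the gap between StartTime and the current time into whole seconds, stores it in TimeValue and creates the timer.
; UpdateText runs the parent formatting, then trims the counter text to its last five characters.
; The event graph holds only disabled placeholder nodes.
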(fn `SetTimerTimeAndStart`
  (params (StartTime :type "DateTime Structure"))
  (set `self.TimeValue` (`KismetMathLibrary.FTrunc` (`KismetMathLibrary.GetTotalSeconds` (- StartTime (`KismetMathLibrary.Now`)))))
  (`self.Create Timer`))

(fn `UpdateText`
  (params (Jump :type Integer) (FinalText :type String))
  (bind _textcounter (`self.TextCounter`))
  (`parent.UpdateText` Jump FinalText)
  (set `Text3DComponent.Text` (`KismetTextLibrary.Conv_StringToText` (`KismetStringLibrary.Right` (`KismetTextLibrary.Conv_TextToString` (`Text3DComponent.Text` _textcounter)) 5)) _textcounter))

(fn `UserConstructionScript`
  (`parent.UserConstructionScript`))