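; BP_configCourse is a race configuration actor meant to display the selected contest (XP, XPS or XPS relais).
; On BeginPlay it creates a dynamic instance of M_Contest, switches on ContestID to set the TextureContest parameter, and prints the contest name.
; The material instance is not assigned to any component in this graph.
; A second ContestID switch is empty, and a StageID switch is left unconnected.
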(event `self.ReceiveBeginPlay`
  (`|ExecutionSequence`
    (:`then_0`
      ;[1 1 1] Afficher le contest choisi
      (bind _returnvalue (`KismetMaterialLibrary.CreateDynamicMaterialInstance` "/Game/Yotta/Material/M_Contest.M_Contest"))
      (switch `int` (`self.ContestID`)
        (:`1`
          (`MaterialInstanceDynamic.SetTextureParameterValue` _returnvalue "TextureContest" "/Game/Yotta/Material/Texture/Stream_-_yottaxp.Stream_-_yottaxp")
          (`KismetSystemLibrary.PrintString` "XP"))
        (:`2`
          (`MaterialInstanceDynamic.SetTextureParameterValue` _returnvalue "TextureContest" "/Game/Yotta/Material/Texture/Stream_-_yottaxps.Stream_-_yottaxps")
          (`KismetSystemLibrary.PrintString` "XPS"))
        (:`3`
          (`MaterialInstanceDynamic.SetTextureParameterValue` _returnvalue "TextureContest" "/Game/Yotta/Material/Texture/Stream_-_yottaxpsrelais.Stream_-_yottaxpsrelais")
          (`KismetSystemLibrary.PrintString` "XPS relais"))))
    (:`then_1`
      (switch `int` (`self.ContestID`)))))

(fn `UserConstructionScript`)